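; NPC actor that runs a short cutscene with a dialog when the player overlaps it.
; BeginPlay creates a player for the NPCcut level sequence.
; Any overlap first turns off the actor's collision; if it is the player, input is disabled, the sequence plays and a Dialog widget appears.
; After a fixed Delay, independent of the sequence's length, the widget is removed and input restored.
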(event EventBeginPlay
  (bind _returnvalue (Sequencer|Player|CreateLevelSequencePlayer "/Game/Blueprints/NPCcut.NPCcut"))
  (Variables|Default|SetSwitch01Cutscene _returnvalue))

(event Collision|EventActorBeginOverlap
  (params (OtherActor :type Actor%20Object%20Reference))
  (bind _returnvalue (Game|GetPlayerCharacter 0))
  (bind _returnvalue_2 (Game|GetPlayerController 0))
  (Collision|SetActorEnableCollision false)
  (if (== OtherActor (Game|GetPlayerCharacter 0))
    (Input|DisableInput _returnvalue _returnvalue_2)
    (Sequencer|Player|Play (Variables|Default|GetSwitch01Cutscene) :!class /Script/MovieScene.MovieSceneSequencePlayer)
    (bind _returnvalue_3 (UserInterface|CreateWidget "/Game/Blueprints/Dialog.Dialog_C" _returnvalue_2))
    (bind _output_get (Variables|Default|SetMyDialogWindow _returnvalue_3))
    (UserInterface|Viewport|AddtoViewport _output_get 0)
    (Utilities|FlowControl|Delay 3.0)
    (Widget|RemovefromParent (Variables|Default|GetMyDialogWindow))
    (Input|EnableInput _returnvalue _returnvalue_2)))

(fn ConstructionScript)